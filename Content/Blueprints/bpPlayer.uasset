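; Player actor for a swipe-controlled maze game that slides along screen X or Z until it hits something.
; While stationary, a touch swipe past a threshold starts movement and counts toward the GameMode's limit, which triggers the defeat menu.
; Tick drives swept moves; hits reset the swipe, shake the camera and allow idle squashing.
; Leaving view outside MainMenu loads the next numbered maze, carrying the swipe through the GameInstance so motion continues.
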(event OnComponentHit(CapsuleComponent)
  (params (HitComponent :type Primitive%20Component%20Object%20Reference) (OtherActor :type Actor%20Object%20Reference) (OtherComp :type Primitive%20Component%20Object%20Reference) (NormalImpulse :type Vector :default "0, 0, 0") (Hit :type Hit%20Result%20Structure%20%28by%20ref%29))
  (Variables|Default|SetMoving false)
  (Utilities|ResetTouch
    (:End
      (Camera|PlayWorldCameraShake "/Game/Blueprints/bpCamShake.bpCamShake_C" (Transformation|GetActorLocation) 0.0 1e+03))))

(event Custom|IdleAnim
  (bind _newtrack_0 (Timeline|Timeline_0 Play)
    (:Update
      (Transformation|SetActorScale3D (Math|Vector|Lerp(Vector) "1.000000,1.000000,1.000000" "0.500000,1.000000,0.500000" _newtrack_0)))))

(event EventBeginPlay
  (bind _asbp_game_mode (Utilities|Casting|CastTobpGameMode (Game|GetGameMode)))
  (Variables|Default|SetGameMode _asbp_game_mode)
  (bind _asbp_game_instance (Utilities|Casting|CastTobpGameInstance (Game|GetGameInstance)))
  (Variables|Default|SetSwipe (Variables|/Game/Blueprints/bpGameInstance.bpGameInstance_C|GetLastSwipe _asbp_game_instance))
  (Variables|Default|SetMoving true)
  (bind _returnvalue (UserInterface|CreateWidget "/Game/Blueprints/Interface/bpOverlay.bpOverlay_C"))
  (UserInterface|Viewport|AddtoViewport _returnvalue 0)
  (Variables|/Script/Engine.PlayerController|SetbShowMouseCursor (Game|GetPlayerController 0) true))

(event Collision|EventActorBeginOverlap
  (params (OtherActor :type Actor%20Object%20Reference)))

(event EventTick
  (params (DeltaSeconds :type Float%20%28single-precision%29))
  (if (Variables|Default|GetMoving)
    (CallFunction|Move)
    (bind _returnvalue (Game|GetCurrentLevelName true))
    (if (not (or (Utilities|Enum|Equal(Enum) _returnvalue "MainMenu") (Class|Actor|WasRecentlyRendered 0.5)))
      (bind _asbp_game_instance (Utilities|Casting|CastTobpGameInstance (Game|GetGameInstance)))
      (Variables|/Game/Blueprints/bpGameInstance.bpGameInstance_C|SetLastSwipe _asbp_game_instance (Variables|Default|GetSwipe))
      (bind _result (Math|Integer|IncrementInt (Variables|/Game/Blueprints/bpGameInstance.bpGameInstance_C|GetCurrentLevel _asbp_game_instance))
        (:%20%20
          (bind _output_get (Variables|/Game/Blueprints/bpGameInstance.bpGameInstance_C|SetCurrentLevel _asbp_game_instance _result))
          (Game|OpenLevel(byName) (Utilities|String|StringToName (Utilities|String|Append "Maze_" (Utilities|String|ToString(Integer) _output_get)))))))
    (else
      (CallFunction|IdleAnim))))

(event Input|ActionEvents|InputActionSwipe
  (params (Key :type Key%20Structure))
  (bind _returnvalue (Game|GetPlayerController 0))
  (bind _returnvalue_2 (Game|GetPlayerController 0))
  (bind _gamemode (Variables|Default|GetGameMode))
  (bind (_locationx _locationy) (Class|PlayerController|GetInputTouchState _returnvalue_2 "Touch1"))
  (bind (_locationx_2 _locationy_2) (Class|PlayerController|GetInputTouchState _returnvalue "Touch1"))
  ;[1 1 1] Input
  (:Pressed
    (if (Variables|Default|GetTakeInput)
      (if (not (Variables|Default|GetMoving))
        (Variables|Default|SetStartTouch (Math|Vector2D|MakeVector2D _locationx_2 _locationy_2)))))
  (:Released
    (if (Variables|Default|GetTakeInput)
      (if (not (Variables|Default|GetMoving))
        (Variables|Default|SetEndTouch (Math|Vector2D|MakeVector2D _locationx _locationy))
        (if (and (Math|Vector|NotEqual(Vector) :A (Variables|Default|GetStartTouch) :ErrorTolerance 0.001) (Math|Vector|NotEqual(Vector) (Variables|Default|GetEndTouch) "(X=0.000000,Y=0.000000)" 0.001))
          (Variables|Default|SetSwipe (- (Variables|Default|GetEndTouch) (Variables|Default|GetStartTouch)))
          (if (or (>= (Math|Float|Absolute(Float) (.x (Variables|Default|GetSwipe))) (Variables|Default|GetSwipeThreshold)) (>= (Math|Float|Absolute(Float) (.y (Variables|Default|GetSwipe))) (Variables|Default|GetSwipeThreshold)))
            (Variables|Default|SetMoving true)
            (Default|AddSwipe _gamemode)
            (if (>= (Variables|/Game/Blueprints/bpGameMode.bpGameMode_C|GetnumSwipes _gamemode) (Variables|/Game/Blueprints/bpGameMode.bpGameMode_C|GetmaxSwipes _gamemode))
              (bind _returnvalue_3 (UserInterface|CreateWidget "/Game/Blueprints/Interface/bpDefeatMenu.bpDefeatMenu_C"))
              (UserInterface|Viewport|AddtoViewport _returnvalue_3 0)
              (Variables|Default|SetTakeInput false))))))))

(fn ConstructionScript)

(fn Move
  (bind _swipe (Variables|Default|GetSwipe))
  (bind _returnvalue (Math|Vector2D|Normalize2D _swipe))
  (Audio|Components|Audio|Stop (Variables|Default|GetTimeline_0))
  (Components|Activation|Activate (Variables|Default|GetTrail) false)
  (Math|Float|CompareFloat (Math|Float|Absolute(Float) (.x _returnvalue)) (Math|Float|Absolute(Float) (.y _returnvalue))
    (:>
      (if (> (.x (Variables|Default|GetSwipe)) 0.0)
        (Transformation|SetActorLocationAndRotation (+ (Transformation|GetActorLocation) (Math|Vector|MakeVector (* (.x (Math|Vector2D|Normalize2D (Variables|Default|GetSwipe))) (Variables|Default|GetSpeed)) 0.0 0.0)) "10.000000, 0, 0" true)
        (else
          (Transformation|SetActorLocationAndRotation (+ (Transformation|GetActorLocation) (Math|Vector|MakeVector (* (.x (Math|Vector2D|Normalize2D (Variables|Default|GetSwipe))) (Variables|Default|GetSpeed)) 0.0 0.0)) "10.000000,180.000000, 0" true))))
    (:<
      (if (> (.y (Variables|Default|GetSwipe)) 0.0)
        (Transformation|SetActorLocationAndRotation (+ (Transformation|GetActorLocation) (Math|Vector|MakeVector 0.0 0.0 (* (* (.y (Math|Vector2D|Normalize2D (Variables|Default|GetSwipe))) -1.0) (Variables|Default|GetSpeed)))) "-80.000000,0.000000,0.000000" true)
        (else
          (Transformation|SetActorLocationAndRotation (+ (Transformation|GetActorLocation) (Math|Vector|MakeVector 0.0 0.0 (* (* (.y (Math|Vector2D|Normalize2D (Variables|Default|GetSwipe))) -1.0) (Variables|Default|GetSpeed)))) "80.000000,0.000000,0.000000" true))))))